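; BP_Turret is a turret that detects the third-person character through PawnSensing, tracks it and fires projectiles at it.
; Each sighting stores the target and sets a looping FireRate timer, while Tick turns the Body toward the target in pitch and yaw.
; The timer spawns BP_Projectile at the Arrow's transform or drops targets beyond SightRadius.
; The timer is never cleared, so without a target it prints an out-of-range message.
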(event `self.ReceiveTick`
  (params (DeltaSeconds :type "Float (single-precision)"))
  (bind (_returnvalue_roll _returnvalue_pitch _returnvalue_yaw) (`KismetMathLibrary.BreakRotator` (`KismetMathLibrary.FindLookAtRotation` (`SceneComponent.K2_GetComponentLocation` (`self.Body`)) (`self.K2_GetActorLocation` (`self.TargetPlayer`)))))
  (if (`KismetSystemLibrary.IsValid` (`self.TargetPlayer`))
    (`SceneComponent.K2_SetWorldRotation` (`self.Body`) (`KismetMathLibrary.MakeRotator` 0.0 _returnvalue_pitch _returnvalue_yaw) false false)))

(event `self.PawnSensing.OnSeePawn`
  (params (Pawn :type "Pawn Object Reference"))
  (bind _asbp_third_person_character (cast `/Game/ThirdPerson/Blueprints/BP_ThirdPersonCharacter` Pawn))
  (set `self.TargetPlayer` _asbp_third_person_character)
  (`KismetSystemLibrary.K2_SetTimerDelegate` (delegate `FireProjectile`) (`self.FireRate`) true))

(event `FireProjectile`
  (bind _targetplayer (`self.TargetPlayer`))
  (bind (_returnvalue_location _returnvalue_rotation) (`KismetMathLibrary.BreakTransform` (`SceneComponent.K2_GetComponentToWorld` (`self.Arrow`))))
  (if (`KismetSystemLibrary.IsValid` _targetplayer)
    (if (> (`self.GetDistanceTo` _targetplayer self) (`PawnSensingComponent.SightRadius` (`self.PawnSensing`)))
      (set `self.TargetPlayer` null)
      (else
        (`|SpawnActorFromClass` "/Game/Blueprints/BP_Projectile.BP_Projectile_C" (`KismetMathLibrary.MakeTransform` _returnvalue_location _returnvalue_rotation) "Undefined" "MultiplyWithRoot" null null)))
    (else
      (`KismetSystemLibrary.PrintString` "Player has left range"))))

(fn `UserConstructionScript`)