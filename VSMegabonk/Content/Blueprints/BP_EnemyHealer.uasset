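; BP_EnemyHealer is a stationary character that periodically heals nearby enemies.
; On BeginPlay it deactivates CharacterMovement and starts a looping timer for HealTick.
; Each tick scans all BP_Enemy actors and sends those within a fixed radius negative damage through ApplyDamage, so healing reuses the damage path.
; It prints each returned damage value to the screen.
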(event `self.ReceiveBeginPlay`
  (`|ExecutionSequence`
    (:`then_0`
      (`ActorComponent.Deactivate` (`self.CharacterMovement`)))
    (:`then_1`
      (`KismetSystemLibrary.K2_SetTimerDelegate` (delegate `HealTick`) 2.0 true))))

(event `HealTick`
  (bind _outactors (`GameplayStatics.GetAllActorsOfClass` "/Game/Blueprints/BP_Enemy.BP_Enemy_C"))
  (for _array_element _outactors
    (if (<= (`self.GetDistanceTo` _array_element self) 1112.0)
      (bind _returnvalue (`GameplayStatics.ApplyDamage` _array_element -25.0 null null "/Script/Engine.DamageType"))
      (`KismetSystemLibrary.PrintString` (`KismetStringLibrary.Conv_DoubleToString` _returnvalue)))))

(fn `UserConstructionScript`
  (`parent.UserConstructionScript`))