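; BP_UpgradeSystem applies data-driven upgrades to the player character's Garlic.
; Its Upgrade event reads the Garlic row from DT_Upgrades and looks up the character's current Level in that row's LevelMap.
; The matching entry sets the Garlic's damage and world scale, with debug prints for found and missing rows.
; Garlic is the only upgrade handled, and NewFunction is an empty stub.
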(event `Upgrade`
  (params (Garlic :type Name))
  ; Upgrading Garlic
  (bind _returnvalue (`|GetDataTableRow` "/Game/Blueprints/DT_Upgrades.DT_Upgrades" Garlic)
    (:`then`
      (bind _asbp_third_person_character (cast `/Game/ThirdPerson/Blueprints/BP_ThirdPersonCharacter` (`GameplayStatics.GetPlayerCharacter` 0)))
      (bind (_damage _size) (break `/Game/Blueprints/GarlicUpgrade` (`BlueprintMapLibrary.Map_Find` (`.LevelMap_14_002CB203404D4C29A6EA8598096D14B8` (break `/Game/Blueprints/Itemupgrade` _returnvalue)) (`/Game/ThirdPerson/Blueprints/BP_ThirdPersonCharacter.Level` _asbp_third_person_character))))
      (bind _garlic (`/Game/ThirdPerson/Blueprints/BP_ThirdPersonCharacter.Garlic` _asbp_third_person_character))
      (set `/Game/Blueprints/BPC_Garlic.Damage` _damage _garlic)
      (`SceneComponent.SetWorldScale3D` _garlic _size)
      (`KismetSystemLibrary.PrintString` "Upgraded"))
    (:`RowNotFound`
      (`KismetSystemLibrary.PrintString` "canada"))))

(fn `NewFunction`)