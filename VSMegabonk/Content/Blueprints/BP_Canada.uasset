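; BP_Canada is a slow field that drags the third-person character's walk speed down while inside its sphere.
; Sphere overlap stores the character reference, and Tick then steps MaxWalkSpeed toward zero at a constant interpolation rate, printing it for debug.
; A delayed Tick branch restores normal speed once it has reached near zero.
; Leaving the sphere restores normal speed immediately and clears the reference.
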(event `self.Sphere.OnComponentBeginOverlap`
  (params (OverlappedComponent :type "PrimitiveComponent Object Reference") (OtherActor :type "Actor Object Reference") (OtherComp :type "PrimitiveComponent Object Reference") (OtherBodyIndex :type Integer) (bFromSweep :type Boolean) (SweepResult :type "HitResult Structure (by ref)"))
  ; Referencing PlayerCharacter
  (bind _asbp_third_person_character (cast `/Game/ThirdPerson/Blueprints/BP_ThirdPersonCharacter` OtherActor))
  (set `self.As BP Third Person Character` _asbp_third_person_character))

(event `self.ReceiveTick`
  (params (DeltaSeconds :type "Float (single-precision)"))
  (bind _as_bp_third_person_character (`self.As BP Third Person Character`))
  (bind _returnvalue (`self.GetComponentByClass` _as_bp_third_person_character "/Script/Engine.CharacterMovementComponent"))
  ; Slowing Player Down when colliding with slowfield
  (`|ExecutionSequence`
    (:`then_0`
      (`/Engine/EditorBlueprintResources/StandardMacros.IsValid` _as_bp_third_person_character
        (:`Is Valid`
          (set `self.IsColliding` true)
          (bind _output_get (set `CharacterMovementComponent.MaxWalkSpeed` (`KismetMathLibrary.FInterpTo_Constant` (`MovementComponent.GetMaxSpeed` _returnvalue) 0.0 DeltaSeconds 150.0) _returnvalue))
          (`KismetSystemLibrary.PrintString` (`KismetStringLibrary.Conv_DoubleToString` _output_get))
          (set `self.MaxSpeed0` (`KismetMathLibrary.NearlyEqual_FloatFloat` _output_get 0.0 0.1)))))
    (:`then_1`
      (`KismetSystemLibrary.Delay` 2.0)
      (if (`self.MaxSpeed0`)
        (set `CharacterMovementComponent.MaxWalkSpeed` 600.0 (`self.GetComponentByClass` (`self.As BP Third Person Character`) "/Script/Engine.CharacterMovementComponent"))
        (`KismetSystemLibrary.PrintString` "Set max speed back to normal")))))

(event `self.Sphere.OnComponentEndOverlap`
  (params (OverlappedComponent :type "PrimitiveComponent Object Reference") (OtherActor :type "Actor Object Reference") (OtherComp :type "PrimitiveComponent Object Reference") (OtherBodyIndex :type Integer))
  ; Resetting Speed
  (set `self.IsColliding` false)
  (bind _asbp_third_person_character (cast `/Game/ThirdPerson/Blueprints/BP_ThirdPersonCharacter` OtherActor))
  (set `CharacterMovementComponent.MaxWalkSpeed` 600.0 (`self.GetComponentByClass` _asbp_third_person_character "/Script/Engine.CharacterMovementComponent"))
  (set `self.As BP Third Person Character` null))

(fn `UserConstructionScript`)