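; BPC_Garlic is a damage-aura component that repeatedly hurts BP_Enemy actors overlapping it.
; On BeginPlay it reads the Garlic row of DT_Upgrades and uses the player character's Level to look up its world scale and damage.
; A short looping timer applies that damage to every overlapping enemy and prints the result.
; The stats are read only at BeginPlay, so later level changes are not picked up here.
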(event `self.ReceiveBeginPlay`
  ;[0.784 0 0 0.5] Damage Event For Garlic
  (`|ExecutionSequence`
    (:`then_0`
      (bind _asbp_third_person_character (cast `/Game/ThirdPerson/Blueprints/BP_ThirdPersonCharacter` (`GameplayStatics.GetPlayerCharacter` 0)))
      (bind _returnvalue (`|GetDataTableRow` "/Game/Blueprints/DT_Upgrades.DT_Upgrades" "Garlic")
        (:`then`
          (bind (_damage _size) (break `/Game/Blueprints/GarlicUpgrade` (`BlueprintMapLibrary.Map_Find` (`.LevelMap_14_002CB203404D4C29A6EA8598096D14B8` (break `/Game/Blueprints/Itemupgrade` _returnvalue)) (`/Game/ThirdPerson/Blueprints/BP_ThirdPersonCharacter.Level` _asbp_third_person_character))))
          (`self.SetWorldScale3D` _size)
          (set `self.Damage` _damage))
        (:`RowNotFound`
          (`KismetSystemLibrary.PrintString` "canada"))))
    (:`then_1`
      (`KismetSystemLibrary.K2_SetTimerDelegate` (delegate `DamageTick`) 0.25 true))))

(event `DamageTick`
  ;[0.784 0 0 0.5] Damage Event For Garlic
  (for _array_element (`self.GetOverlappingActors` "/Game/Blueprints/BP_Enemy.BP_Enemy_C")
    (bind _returnvalue (`GameplayStatics.ApplyDamage` _array_element (`self.Damage`) null null "/Script/Engine.DamageType"))
    (`KismetSystemLibrary.PrintString` (`KismetStringLibrary.Conv_DoubleToString` _returnvalue))))