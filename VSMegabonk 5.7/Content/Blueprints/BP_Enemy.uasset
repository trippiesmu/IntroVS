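; BP_Enemy is an enemy that chases the player, deals contact damage and drops XP when killed.
; PawnSensing sets a seen flag, which is never cleared here, and starts an AI move toward the player character.
; A looping timer damages third-person characters overlapping its capsule.
; Incoming damage lowers Health, shown on a widget healthbar updated every Tick; at zero it destroys itself and spawns BP_xp at its location.
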(event `self.ReceiveTick`
  (params (DeltaSeconds :type "Float (single-precision)"))
  ; Updating EnemyHealthbar
  (bind _aswp_enemy_health (cast `/Game/Blueprints/WP_EnemyHealth` (`WidgetComponent.GetWidget` (`self.HealthbarWidget`))))
  (`ProgressBar.SetPercent` (`/Game/Blueprints/WP_EnemyHealth.EnemyHealth` _aswp_enemy_health) (/ (`self.health`) 100.0)))

(event `self.ReceiveAnyDamage`
  (params (Damage :type "Float (single-precision)") (DamageType :type "DamageType Object Reference") (InstigatedBy :type "Controller Object Reference") (DamageCauser :type "Actor Object Reference"))
  ; Receiving Damage
  (set `self.health` (- (`self.health`) Damage))
  (if (<= (`self.health`) 0.0)
    (`self.K2_DestroyActor`)
    (`KismetSystemLibrary.PrintString` "Enemy Killed")
    (bind _returnvalue (`|SpawnActorFromClass` "/Game/Blueprints/BP_xp.BP_xp_C" (`KismetMathLibrary.MakeTransform` (`self.K2_GetActorLocation`)) "Undefined" "MultiplyWithRoot" null null))
    (`KismetSystemLibrary.PrintString` (`KismetSystemLibrary.GetDisplayName` _returnvalue))))

(event `self.PawnSensing.OnSeePawn`
  (params (Pawn :type "Pawn Object Reference"))
  ; Checking if the enemy is seeing the Player
  (set `self.IsSeeingPlayer` true)
  (`self.FollowPlayer`))

(event `FollowPlayer`
  ; Make the enemy follow the player
  (if (`self.IsSeeingPlayer`)
    (`|AIMoveTo` self (0.0 0.0 0.0) (`GameplayStatics.GetPlayerCharacter` 0) 50.0)))

(event `self.ReceiveBeginPlay`
  ; Doing Damage to Player
  (`KismetSystemLibrary.K2_SetTimerDelegate` (delegate `DamageTick`) 0.5 true))

(event `DamageTick`
  ; Doing Damage to Player
  (for _array_element (`PrimitiveComponent.GetOverlappingActors` (`self.CapsuleComponent`) "/Game/ThirdPerson/Blueprints/BP_ThirdPersonCharacter.BP_ThirdPersonCharacter_C")
    (bind _returnvalue (`GameplayStatics.ApplyDamage` _array_element 5.0 null self "/Script/Engine.DamageType"))
    (`KismetSystemLibrary.PrintString` (`KismetStringLibrary.Conv_DoubleToString` _returnvalue))))

(fn `UserConstructionScript`)